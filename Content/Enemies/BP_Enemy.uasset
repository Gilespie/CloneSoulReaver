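; BP_Enemy is an enemy with a simple health pool that registers itself with GamConditions on BeginPlay and starts at MaxHealth.
; Its TakeDamage event subtracts damage, prints the clamped health as debug text, and at zero unregisters the enemy and destroys the actor.
; An IsAlive helper tests for health at or above zero, but TakeDamage ignores its result and does its own death check.
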(event EventBeginPlay
  (bind _output_get (Variables|Default|SetCurrentHealth (Variables|Default|GetMaxHealth)))
  (Development|PrintString (Utilities|String|ToString(Float) _output_get))
  (Default|RegisterEnemy (Variables|Default|GetGamConditions) self))

(event EventTakeDamage
  (params (Damage :type Float%20%28double-precision%29))
  ;[0.15 0.15 0.15 0.5] TAKEDAMAGE
  (bind _output_get (Variables|Default|SetCurrentHealth (- (Variables|Default|GetCurrentHealth) Damage)))
  (CallFunction|IsAlive (Math|Float|Clamp(Float) _output_get 0.0 (Variables|Default|GetMaxHealth)))
  (Development|PrintString (Utilities|String|ToString(Float) (Math|Float|Clamp(Float) _output_get 0.0 (Variables|Default|GetMaxHealth))) true true "(R=1.000000,G=0.000000,B=0.189890,A=1.000000)")
  (if (<= (Math|Float|Clamp(Float) _output_get 0.0 (Variables|Default|GetMaxHealth)) 0.0)
    (Variables|Default|SetCurrentHealth 0.0)
    (Development|PrintString "Dead!")
    (Default|UnregisterEnemy (Variables|Default|GetGamConditions) self)
    (Actor|DestroyActor)))

(fn ConstructionScript)

(fn IsAlive
  (params (currentHealth :type Float%20%28double-precision%29))
  (return (>= currentHealth 0.0)))