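; Win condition component that tracks living enemies as a kill objective and triggers the end-of-game screen.
; It binds event dispatchers on BeginPlay to add or remove enemies from an array, sending the remaining count to BP_PC's quest update.
; When a removal empties the array, it fires OnConditionsMeet.
; If Victory is set, that handler shows WBP_GamePanels using the player's IsDead state and switches to UI-only input with a cursor.
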(event Custom|Event_UpdateQuest
  (params (Task :type String) (Count :type Integer) (Target :type String))
  (bind _asbp_pc (Utilities|Casting|CastToBP_PC (Game|GetPlayerController 0))
    (:then
      (Default|UpdateQuest _asbp_pc Task Count Target))
    (:CastFailed
      (Development|PrintString "NOT"))))

(event Custom|RegisterEnemy_Event
  (params (Enemy :type BPC%20Minion%20Component%20Object%20Reference))
  (CallFunction|RegisterEnemy Enemy)
  (Default|CallOnUpdateQuest "Kill:" (CallFunction|GetEnemyCount) "Enemies"))

(event Custom|CheckWinCondition_Event
  (params (Enemy :type BPC%20Minion%20Component%20Object%20Reference))
  (CallFunction|UnregisterEnemy Enemy)
  (Default|CallOnUpdateQuest "Kill:" (CallFunction|GetEnemyCount) "Enemies")
  (CallFunction|CheckWinConditions))

(event Custom|Event_OnConditionsMeet
  (bind _returnvalue (Game|GetPlayerController 0))
  (if (Variables|Default|GetVictory)
    (bind _asbp_third_person_character (Utilities|Casting|CastToBP_ThirdPersonCharacter (Game|GetPlayerCharacter 0)))
    (bind _returnvalue_2 (UserInterface|CreateWidget "/Game/Blueprints/HUDS/WBP_GamePanels.WBP_GamePanels_C" (Game|GetPlayerController 0)))
    (UserInterface|Viewport|AddtoViewport _returnvalue_2 0)
    (Default|ShowResult _returnvalue_2 (Default|IsDead (Variables|/Game/ThirdPerson/BP_ThirdPersonCharacter.BP_ThirdPersonCharacter_C|GetBPC_HealthSystem _asbp_third_person_character)))
    (Input|SetInputModeUIOnly _returnvalue 0 "DoNotLock" false)
    (Variables|/Script/Engine.PlayerController|SetbShowMouseCursor _returnvalue true)))

(event EventBeginPlay
  (EventDispatchers|BindEventtoOnUpdateQuest (delegate Custom|Event_UpdateQuest))
  (EventDispatchers|BindEventtoOnRegisterEnemy (delegate Custom|RegisterEnemy_Event))
  (EventDispatchers|BindEventtoOnWinCondition (delegate Custom|CheckWinCondition_Event))
  (EventDispatchers|BindEventtoOnConditionsMeet (delegate Custom|Event_OnConditionsMeet)))

(fn RegisterEnemy
  (params (Enemy :type BPC%20Minion%20Component%20Object%20Reference%20%28by%20ref%29))
  (Utilities|Array|Add (Variables|Default|GetEnemies) Enemy))

(fn UnRegisterEnemy
  (params (Enemy :type BPC%20Minion%20Component%20Object%20Reference%20%28by%20ref%29))
  (Utilities|Array|RemoveItem (Variables|Default|GetEnemies) Enemy))

(fn CheckWinConditions
  (if (not (> (Utilities|Array|Length (Variables|Default|GetEnemies)) 0))
    (Default|CallOnConditionsMeet)))

(fn GetEnemyCount
  (return (Utilities|Array|Length (Variables|Default|GetEnemies))))