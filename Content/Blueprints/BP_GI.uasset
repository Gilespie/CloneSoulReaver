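; Game instance that holds the game's difficulty and carries player, boss and minion state through save slots.
; On init it looks up the selected difficulty's row in a data table and caches it as GameDifficult.
; SaveToSlot writes that state and the current level into a new BP_SaveData.
; LoadFromSlot restores it, except boss health, sets IsLoaded and opens the saved level, without reapplying the difficulty row.
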(event EventInit
  (CallFunction|ApplyDifficulty))

(fn GetRowName
  (params (Difficult :type EDifficult%20Enum :default "NewEnumerator0"))
  (return (Utilities|Select :Index Difficult :NewEnumerator0 "Easy" :NewEnumerator1 "Medium" :NewEnumerator2 "Hard")))

(fn ApplyDifficulty
  (bind _returnvalue (Utilities|GetDataTableRow "/Game/Blueprints/DT_SDifficultData.DT_SDifficultData" (CallFunction|GetRowName (Variables|Default|GetDifficult)))
    (:then
      (Variables|Default|SetGameDifficult _returnvalue))))

(fn SavetoSlot
  (params (SlotName :type String) (SOURCE :type String))
  (bind _gisavedminions (Variables|Default|GetGISavedMinions))
  (Development|PrintString (Utilities|String|Append "SaveToSlot || " "Called From >> " SOURCE) true true "(R=1.000000,G=1.000000,B=0.000000,A=1.000000)")
  (bind _returnvalue (SaveGame|DoesSaveGameExist SlotName))
  (bind _returnvalue_2 (SaveGame|CreateSaveGameObject "/Game/Blueprints/BP_SaveData.BP_SaveData_C"))
  (bind _output_get (Variables|Default|SetSaveData _returnvalue_2))
  (Variables|/Game/Blueprints/BP_SaveData.BP_SaveData_C|SetPlayerPos _output_get (Variables|Default|GetPlayerPos))
  (Variables|/Game/Blueprints/BP_SaveData.BP_SaveData_C|SetPlayerHealth _output_get (Variables|Default|GetPlayerHealth))
  (Variables|/Game/Blueprints/BP_SaveData.BP_SaveData_C|SetDifficult _output_get (Variables|Default|GetDifficult))
  (Variables|/Game/Blueprints/BP_SaveData.BP_SaveData_C|SetBossPhase _output_get (Variables|Default|GetBossPhase))
  (Variables|/Game/Blueprints/BP_SaveData.BP_SaveData_C|SetBossHealth _output_get (Variables|Default|GetBossHealth))
  (Variables|/Game/Blueprints/BP_SaveData.BP_SaveData_C|SetSavedMinionIndex _output_get _gisavedminions)
  (bind _returnvalue_3 (Game|GetCurrentLevelName true))
  (bind _output_get_2 (Variables|/Game/Blueprints/BP_SaveData.BP_SaveData_C|SetLevel _output_get (Utilities|String|StringToName _returnvalue_3)))
  (SaveGame|SaveGametoSlot _output_get SlotName)
  (Development|PrintString (Utilities|String|Append (Utilities|String|Append "BPGI > SAVED SLOT: " SlotName) (Utilities|String|Append "|| PLAYER HP: " (Utilities|String|ToString(Float) (Variables|Default|GetPlayerHealth))) (Utilities|String|Append "|| PLAYER POS: " (Utilities|String|ToString(Vector) (Variables|Default|GetPlayerPos))) (Utilities|String|Append "|| DIFFICULTY: " (Utilities|String|EnumtoString (Variables|Default|GetDifficult))) (Utilities|String|Append "|| BOSS PHASE: " (Utilities|String|EnumtoString (Variables|Default|GetBossPhase))) (Utilities|String|Append "|| Level: " (Utilities|String|ToString(Name) _output_get_2)) (Utilities|String|Append "|| Boss HP: " (Utilities|String|ToString(Float) (Variables|Default|GetBossHealth))) (Utilities|String|Append "|| CURRENT ENEMIES: " (Utilities|String|ToString(Integer) (Utilities|Array|Length _gisavedminions)))) true true "(R=1.000000,G=1.000000,B=0.000000,A=1.000000)"))

(fn LoadfromSlot
  (params (SlotName :type String))
  (Development|PrintString (Utilities|String|Append "LOADED SLOT >> " SlotName))
  (bind _returnvalue (SaveGame|LoadGamefromSlot SlotName))
  (bind _asbp_save_data (Utilities|Casting|CastToBP_SaveData _returnvalue))
  (Utilities|IsValid _asbp_save_data
    (:Is%20Valid
      (bind _returnvalue_2 (SaveGame|DoesSaveGameExist SlotName))
      (if _returnvalue_2
        (Variables|Default|SetSaveData _asbp_save_data)
        (Variables|Default|SetIsLoaded true)
        (Variables|Default|SetDifficult (Variables|/Game/Blueprints/BP_SaveData.BP_SaveData_C|GetDifficult _asbp_save_data))
        (Variables|Default|SetPlayerHealth (Variables|/Game/Blueprints/BP_SaveData.BP_SaveData_C|GetPlayerHealth _asbp_save_data))
        (Variables|Default|SetLevel (Variables|/Game/Blueprints/BP_SaveData.BP_SaveData_C|GetLevel _asbp_save_data))
        (bind _output_get (Variables|Default|SetGISavedMinions (Variables|/Game/Blueprints/BP_SaveData.BP_SaveData_C|GetSavedMinionIndex _asbp_save_data)))
        (Development|PrintString (Utilities|String|Append "Loaded Minions >> " (Utilities|String|ToString(Integer) (Utilities|Array|Length _output_get))) true true "(R=1.000000,G=1.000000,B=0.000000,A=1.000000)")
        (Variables|Default|SetBossPhase (Variables|/Game/Blueprints/BP_SaveData.BP_SaveData_C|GetBossPhase _asbp_save_data))
        (Variables|Default|SetPlayerPos (Variables|/Game/Blueprints/BP_SaveData.BP_SaveData_C|GetPlayerPos _asbp_save_data))
        (Game|OpenLevel(byName) (Variables|Default|GetLevel))))
    (:Is%20Not%20Valid
      (Development|PrintString "NOT VALID" true true "(R=1.000000,G=0.000000,B=0.000000,A=1.000000)" 5.0))))