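; Meteor storm hazard area that rains projectiles once its linked boss triggers the OnMeteorStorm event.
; BeginPlay hides the RectLight and binds to the boss event, which permanently sets the storm active.
; While active and the boss is alive, Tick shows the light and runs a cooldown timer, spawning a projectile at a random X/Y point within the Box on each expiry.
; Spawning stops on boss death, but the light is never hidden again.
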(event Custom|OnMeteorStorm
  (Variables|Default|SetIsActive true))

(event EventBeginPlay
  (CallFunction|ResetTimer)
  (Rendering|SetVisibility (Variables|Default|GetRectLight) false false)
  (EventDispatchers|BindEventtoOnMeteorStorm (Variables|Default|GetBossPrefab) (delegate Custom|OnMeteorStorm)))

(event EventTick
  (params (DeltaSeconds :type Float%20%28single-precision%29))
  (if (and (Variables|Default|GetIsActive) (not (Default|IsDead (Variables|/Game/Actors/Boss/BP_Boss.BP_Boss_C|GetBPC_HealthSystem (Variables|Default|GetBossPrefab)))))
    (Rendering|SetVisibility (Variables|Default|GetRectLight) true false)
    (bind _output_get (Variables|Default|Settimer (- (Variables|Default|Gettimer) DeltaSeconds)))
    (if (<= _output_get 0.0)
      (CallFunction|Spawn)
      (CallFunction|ResetTimer))))

(fn ConstructionScript)

(fn Spawn
  (bind _box (Variables|Default|GetBox))
  (bind _returnvalue (Components|Box|GetScaledBoxExtent _box))
  (bind _result (Math|Float|NegateFloat (.x _returnvalue))
    (:%20%20
      (bind _result_2 (Math|Float|NegateFloat (.y _returnvalue))
        (:%20%20
          (Game|SpawnActorfromClass (Variables|Default|GetProjectile) (Math|Conversions|ToTransform(Vector) (Math|Transform|TransformLocation (Transformation|GetWorldTransform (Variables|Default|GetBox)) (Math|Vector|MakeVector (Math|Random|RandomFloatinRange _result (.x _returnvalue)) (Math|Random|RandomFloatinRange _result_2 (.y _returnvalue)) (Math|Random|RandomFloatinRange 0.0 0.0)))) "Undefined" "MultiplyWithRoot" 0 0))))))

(fn ResetTimer
  (Variables|Default|Settimer (Variables|Default|GetCooldown)))