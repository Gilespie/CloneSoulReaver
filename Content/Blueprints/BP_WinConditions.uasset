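; BP_WinConditions tracks the level's enemies and keeps the player's quest display updated with how many remain.
; On BeginPlay it binds to register and win-condition events, which add or remove enemies from an array.
; Each event passes the new count to BP_PC's UpdateQuest, and each removal plays a camera shutter sound.
; CheckWinCondition only tests whether enemies remain, with no win outcome implemented.
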(event Custom|CheckWinCondition_Event
  (params (Enemy :type BPC%20Minion%20Component%20Object%20Reference))
  (CallFunction|UnregisterEnemy Enemy)
  (bind _asbp_pc (Utilities|Casting|CastToBP_PC (Game|GetPlayerController 0)))
  (Default|UpdateQuest _asbp_pc (CallFunction|GetEnemyCount))
  (CallFunction|CheckWinCondition))

(event Custom|RegisterEnemy_Event
  (params (Enemy :type BPC%20Minion%20Component%20Object%20Reference))
  (CallFunction|RegisterEnemy Enemy)
  (bind _asbp_pc (Utilities|Casting|CastToBP_PC (Game|GetPlayerController 0))
    (:then
      (Default|UpdateQuest _asbp_pc (CallFunction|GetEnemyCount)))
    (:CastFailed
      (Development|PrintString "NOT"))))

(event EventBeginPlay
  (EventDispatchers|BindEventtoOnRegisterEnemy (delegate Custom|RegisterEnemy_Event))
  (EventDispatchers|BindEventtoOnWinCondition (delegate Custom|CheckWinCondition_Event)))

(fn ConstructionScript)

(fn RegisterEnemy
  (params (Enemy :type BPC%20Minion%20Component%20Object%20Reference))
  (Utilities|Array|Add (Variables|Default|GetEnemies) Enemy))

(fn UnregisterEnemy
  (params (Enemy :type BPC%20Minion%20Component%20Object%20Reference))
  (Utilities|Array|RemoveItem (Variables|Default|GetEnemies) Enemy)
  (Audio|PlaySound2D "/Engine/VREditor/Sounds/UI/Camera_Shutter.Camera_Shutter" 1.0 1.0 0.0 0 0))

(fn CheckWinCondition
  (if (> (Utilities|Array|Length (Variables|Default|GetEnemies)) 0)
    _))

(fn GetEnemyCount
  (return (Utilities|Array|Length (Variables|Default|GetEnemies))))