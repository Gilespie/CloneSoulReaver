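; Health component that tracks current health, damage and death for whatever it is attached to.
; On BeginPlay it fills health and binds to OnTakeDamage; each hit clamps the new value, plays a 2D sound and prints a debug name.
; Dispatchers broadcast health updates and a one-time death guarded by IsAlive, which ResetValues restores along with full health.
; IsCharacterAlive is unwired, so its health check never runs.
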(event Custom|TakeDamage_Event
  (params (Damage :type Float%20%28double-precision%29))
  (Development|PrintString (Utilities|GetDisplayName self))
  (CallFunction|TakeDamage Damage)
  (Default|CallOnUpdateHealth (Variables|Default|GetCurrentHealth) (Variables|Default|GetMaxHealth))
  (if (Variables|Default|GetIsAlive)
    (if (CallFunction|IsDead)
      (Variables|Default|SetIsAlive false)
      (Default|CallOnDead))))

(event EventBeginPlay
  (Variables|Default|SetCurrentHealth (Variables|Default|GetMaxHealth))
  (EventDispatchers|BindEventtoOnTakeDamage (delegate Custom|TakeDamage_Event)))

(fn IsCharacterAlive)

(fn TakeDamage
  (params (damage :type Float%20%28double-precision%29))
  (Variables|Default|SetCurrentHealth (CallFunction|CalculateDMG damage))
  (Audio|PlaySound2D (Variables|Default|GetHitSound) 1.0 1.0 0.0 0 0))

(fn IsDead
  (return (<= (Variables|Default|GetCurrentHealth) 0.0)))

(fn CalculateDMG
  (params (Damage :type Float%20%28double-precision%29))
  (return (Math|Float|Clamp(Float) (- (Variables|Default|GetCurrentHealth) Damage) 0.0 (Variables|Default|GetMaxHealth))))

(fn ResetValues
  (bind _maxhealth (Variables|Default|GetMaxHealth))
  (bind _output_get (Variables|Default|SetCurrentHealth _maxhealth))
  (Variables|Default|SetIsAlive true)
  (Default|CallOnUpdateHealth _output_get _maxhealth))