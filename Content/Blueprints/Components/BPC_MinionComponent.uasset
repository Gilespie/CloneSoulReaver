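; BPC_MinionComponent is an actor component that registers its owner as an enemy for the win condition.
; On BeginPlay it binds to the owner's BPC_HealthSystem OnDead event, then registers itself with WinCondition one tick later.
; On death it reports the elimination to WinCondition and destroys the owning actor.
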(event Custom|OnDead_Event
  ;[0.15 0.15 0.15 0.5] OnDead
  (Default|CallOnEnemyEliminated (Variables|Default|GetWinCondition) self)
  (Actor|DestroyActor (Components|GetOwner)))

(event EventBeginPlay
  (bind _output_get (Variables|Default|SetHealthSystem (Actor|GetComponentbyClass (Components|GetOwner) "/Game/Blueprints/Components/BPC_HealthSystem.BPC_HealthSystem_C")))
  (Utilities|FlowControl|Sequence
    (:then_0
      (EventDispatchers|BindEventtoOnDead _output_get (delegate Custom|OnDead_Event)))
    (:then_1
      (Utilities|FlowControl|DelayUntilNextTick)
      (Default|CallOnRegisterEnemy (Variables|Default|GetWinCondition) self))))