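; BPC_HealthSystem is a health component that tracks current health and applies incoming damage.
; On BeginPlay it fills health to the maximum and binds a handler to OnTakeDamage, which subtracts damage clamped between zero and max.
; IsCharacterAlive derives the IsAlive flag from health, but the damage handler reads that flag without calling it, and its branch does nothing.
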(event Custom|TakeDamage_Event
  (params (NewParam :type Float%20%28double-precision%29))
  (CallFunction|TakeDamage NewParam)
  (if (Variables|Default|GetIsAlive)
    _))

(event EventBeginPlay
  (Variables|Default|SetCurrentHealth (Variables|Default|GetMaxHealth))
  (EventDispatchers|BindEventtoOnTakeDamage (delegate Custom|TakeDamage_Event)))

(fn IsCharacterAlive
  (bind _output_get (Variables|Default|SetIsAlive (> (Variables|Default|GetCurrentHealth) 0.0)))
  (return _output_get))

(fn TakeDamage
  (params (damage :type Float%20%28double-precision%29))
  (Variables|Default|SetCurrentHealth (Math|Float|Clamp(Float) (- (Variables|Default|GetCurrentHealth) damage) 0.0 (Variables|Default|GetMaxHealth))))