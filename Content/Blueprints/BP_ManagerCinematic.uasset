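; BP_ManagerCinematic is a manager that plays a referenced cinematic sequence once per game instance.
; On BeginPlay it casts the game instance to BP_GI and, if HasPlayedSequence is unset, starts playback and sets that flag, so later BeginPlays skip it.
; The play event runs RefCinematic's sequence player and prints its playing state for debugging, while a failed cast prints an error.
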(event Custom|Event_Play
  (bind _refcinematic (Variables|Default|GetRefCinematic))
  (bind _sequenceplayer (Variables|/Script/LevelSequence.LevelSequenceActor|GetSequencePlayer _refcinematic))
  (Sequencer|Player|Play _sequenceplayer :!class /Script/MovieScene.MovieSceneSequencePlayer)
  (Development|PrintString (Utilities|String|Append "IS PLAYING SEQUENCE: " (Utilities|String|ToString(Boolean) (Audio|Components|Audio|IsPlaying _sequenceplayer))) true true "(R=1.000000,G=1.000000,B=0.000000,A=1.000000)" 5.0))

(event EventBeginPlay
  (bind _asbp_gi (Utilities|Casting|CastToBP_GI (Game|GetGameInstance))
    (:then
      (if (not (Variables|/Game/Blueprints/BP_GI.BP_GI_C|GetHasPlayedSequence _asbp_gi))
        (CallFunction|EventPlay)
        (Variables|/Game/Blueprints/BP_GI.BP_GI_C|SetHasPlayedSequence _asbp_gi true)))
    (:CastFailed
      (Development|PrintString "CAST FAILED"))))

(fn ConstructionScript)