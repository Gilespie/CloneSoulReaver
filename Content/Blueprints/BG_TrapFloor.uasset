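; Trap floor actor whose two halves swing open after the player steps on it.
; When a third-person character enters the Box trigger, a TimeToActivate delay runs before two timelines pitch RotateRight and RotateLeft open.
; When the character leaves, separate close timelines play from start immediately to rotate both halves back, without cancelling any pending opening.
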(event OnComponentBeginOverlap(Box)
  (params (OverlappedComponent :type Primitive%20Component%20Object%20Reference) (OtherActor :type Actor%20Object%20Reference) (OtherComp :type Primitive%20Component%20Object%20Reference) (OtherBodyIndex :type Integer) (bFromSweep :type Boolean) (SweepResult :type Hit%20Result%20Structure%20%28by%20ref%29))
  (Utilities|Casting|CastToBP_ThirdPersonCharacter OtherActor)
  (Utilities|FlowControl|Delay (Variables|Default|GetTimeToActivate))
  (Utilities|FlowControl|Sequence
    (:then_0
      (bind _rotation (Timeline|OpenFloorRight PlayFromStart)
        (:Update
          (Transformation|SetRelativeRotation (Variables|Default|GetRotate_Right) (Math|Rotator|MakeRotator 0.0 _rotation 0.0) false false))))
    (:then_1
      (bind _rotation_2 (Timeline|OpenFloorLeft PlayFromStart)
        (:Update
          (Transformation|SetRelativeRotation (Variables|Default|GetRotate_Left) (Math|Rotator|MakeRotator 0.0 _rotation_2 0.0) false false))))))

(event OnComponentEndOverlap(Box)
  (params (OverlappedComponent :type Primitive%20Component%20Object%20Reference) (OtherActor :type Actor%20Object%20Reference) (OtherComp :type Primitive%20Component%20Object%20Reference) (OtherBodyIndex :type Integer))
  (Utilities|Casting|CastToBP_ThirdPersonCharacter OtherActor)
  (Utilities|FlowControl|Sequence
    (:then_0
      (bind _rotation (Timeline|CloseFloorRight PlayFromStart)
        (:Update
          (Transformation|SetRelativeRotation (Variables|Default|GetRotate_Right) (Math|Rotator|MakeRotator 0.0 _rotation 0.0) false false))))
    (:then_1
      (bind _rotation_2 (Timeline|CloseFloorLeft PlayFromStart)
        (:Update
          (Transformation|SetRelativeRotation (Variables|Default|GetRotate_Left) (Math|Rotator|MakeRotator 0.0 _rotation_2 0.0) false false))))))

(fn ConstructionScript)