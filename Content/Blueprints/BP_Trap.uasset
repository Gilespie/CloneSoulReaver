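; BP_Trap is a trap actor that repeatedly fires BP_Bullet projectiles on a timer.
; Tick accumulates delta time, and once the total reaches FireRate it calls SpawnBullet and resets the total to zero, so FireRate acts as the interval between shots.
; SpawnBullet spawns the given class at the supplied position with the trap's rotation and unit scale.
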(event EventTick
  (params (DeltaSeconds :type Float%20%28single-precision%29))
  (bind _output_get (Variables|Default|SetAcomulatedTime (+ DeltaSeconds (Variables|Default|GetAcomulatedTime))))
  (if (>= _output_get (Variables|Default|GetFireRate))
    (CallFunction|SpawnBullet "/Game/Blueprints/BP_Bullet.BP_Bullet_C" (Transformation|GetActorLocation))
    (Variables|Default|SetAcomulatedTime 0.0)))

(fn ConstructionScript)

(fn SpawnBullet
  (params (Class :type Actor%20Object%20Reference) (SpawnPos :type Vector))
  (Game|SpawnActorfromClass Class (Math|Transform|MakeTransform SpawnPos (Transformation|GetActorRotation)) "Undefined" "MultiplyWithRoot" 0 0))