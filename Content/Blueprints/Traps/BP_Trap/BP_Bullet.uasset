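; BP_Bullet is a trap projectile that damages the third-person player character on overlap.
; Each tick it moves along its forward vector without sweeping, while an accumulated timer destroys it once the delay is reached.
; Player overlaps call the character's health system component directly and leave the bullet alive; overlaps with any other actor destroy it.
; An ApplyDamage node exists but is never executed.
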(event Collision|EventActorBeginOverlap
  (params (OtherActor :type Actor%20Object%20Reference))
  (bind _asbp_third_person_character (Utilities|Casting|CastToBP_ThirdPersonCharacter OtherActor)
    (:then
      (Default|CallOnTakeDamage (Variables|/Game/ThirdPerson/Blueprints/BP_ThirdPersonCharacter.BP_ThirdPersonCharacter_C|GetBPC_HealthSystem _asbp_third_person_character) (Variables|Default|GetDamage)))
    (:CastFailed
      (Actor|DestroyActor))))

(event EventTick
  (params (DeltaSeconds :type Float%20%28single-precision%29))
  (CallFunction|Move (Variables|Default|GetSpeed) DeltaSeconds)
  (bind _istimer (CallFunction|SetTimer DeltaSeconds))
  (if _istimer
    (Variables|Default|SetTimer 0.0)
    (Actor|DestroyActor)))

(fn ConstructionScript)

(fn Move
  (params (moveSpeed :type Float%20%28double-precision%29) (deltaTime :type Float%20%28double-precision%29))
  (Transformation|SetActorLocation (+ (* (* moveSpeed (Transformation|GetActorForwardVector)) deltaTime) (Transformation|GetActorLocation)) false false))

(fn SetTimer
  (params (DeltaSeconds :type Float%20%28double-precision%29))
  (bind _output_get (Variables|Default|SetTimer (+ DeltaSeconds (Variables|Default|GetTimer))))
  (return (>= _output_get (Variables|Default|GetDelay))))