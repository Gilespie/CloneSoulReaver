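; BP_TrapSaw is a moving saw trap that damages the player character on contact.
; Each tick it accumulates time, scales it by a multiplier, wraps it to 0–1 and teleport-free moves itself along the TrapSawPath spline at constant velocity, looping continuously.
; On overlap with BP_ThirdPersonCharacter it calls take-damage on the character's health system; an ApplyDamage node is left unconnected.
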(event Collision|EventActorBeginOverlap
  (params (OtherActor :type Actor%20Object%20Reference))
  (bind _asbp_third_person_character (Utilities|Casting|CastToBP_ThirdPersonCharacter OtherActor))
  (Default|CallOnTakeDamage (Variables|/Game/ThirdPerson/Blueprints/BP_ThirdPersonCharacter.BP_ThirdPersonCharacter_C|GetBPC_HealthSystem _asbp_third_person_character) (Variables|Default|GetDamage)))

(event EventTick
  (params (DeltaSeconds :type Float%20%28single-precision%29))
  (bind _output_get (Variables|Default|SetGameTime (+ DeltaSeconds (Variables|Default|GetGameTime))))
  (Transformation|SetActorLocation (Spline|GetLocationatTime (Variables|/Game/Blueprints/Traps/SawTrap/BP_TrapSawPath.BP_TrapSawPath_C|GetSpline (Variables|Default|GetTrapSawPath)) (Class|KismetMathLibrary|FWrap (* _output_get (Variables|Default|GetMultiplier)) 0.0 1.0) "World" true) false false))

(fn ConstructionScript)