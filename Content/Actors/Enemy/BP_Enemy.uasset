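; BP_Enemy is an enemy actor that registers itself with GameConditions on BeginPlay.
; When its health system fires OnDead, it calls the win-condition event on GameConditions, passing itself, and destroys itself.
; AI perception updates write the sensed actor to the target key in its controller's Blackboard, or clear it when sensing fails.
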(event OnTargetPerceptionUpdated(AIPerception)
  (params (Actor :type Actor%20Object%20Reference) (Stimulus :type AI%20Stimulus%20Structure))
  (AI|Components|Blackboard|SetValueasObject (AI|GetBlackboard (Pawn|GetController)) (Variables|Default|GetTargetKey) (Utilities|SelectObject Actor 0 (.bSuccessfullySensed (Utilities|Struct|BreakAIStimulus Stimulus)))))

(event Custom|OnDead_Event
  ;[0.15 0.15 0.15 0.5] OnDead
  (Default|CallOnWinCondition (Variables|Default|GetGameConditions) self)
  (Actor|DestroyActor))

(event EventBeginPlay
  (Utilities|FlowControl|Sequence
    (:then_0
      (Default|CallOnRegisterEnemy (Variables|Default|GetGameConditions) self))
    (:then_1
      (EventDispatchers|BindEventtoOnDead (Variables|Default|GetBPC_HealthSystem) (delegate Custom|OnDead_Event)))))

(fn ConstructionScript)