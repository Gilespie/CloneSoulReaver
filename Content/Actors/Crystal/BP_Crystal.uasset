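; BP_Crystal is a crystal actor that flies toward the boss and destroys itself on contact.
; On BeginPlay it resolves its Boss reference, using the first BP_Boss in the level if unset, and rotates to face it once.
; While CanMove is true, Tick moves it straight forward at a fixed speed without sweeping or re-aiming.
; A capsule overlap with a BP_Boss destroys the crystal; no damage is applied here.
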(event OnComponentBeginOverlap(Collision_Capsule)
  (params (OverlappedComponent :type Primitive%20Component%20Object%20Reference) (OtherActor :type Actor%20Object%20Reference) (OtherComp :type Primitive%20Component%20Object%20Reference) (OtherBodyIndex :type Integer) (bFromSweep :type Boolean) (SweepResult :type Hit%20Result%20Structure%20%28by%20ref%29))
  (bind _asbp_boss (Utilities|Casting|CastToBP_Boss OtherActor))
  (Utilities|IsValid _asbp_boss
    (:Is%20Valid
      (Actor|DestroyActor))))

(event Custom|Event_SetBossAndLook
  (bind _returnvalue (Transformation|GetActorLocation))
  (Utilities|IsValid (Variables|Default|GetBoss)
    (:Is%20Valid
      (Transformation|SetActorRotation (Math|Rotator|FindLookatRotation _returnvalue (Transformation|GetActorLocation (Variables|Default|GetBoss)))))
    (:Is%20Not%20Valid
      (bind _outactors (Actor|GetAllActorsOfClass "/Game/Actors/Boss/BP_Boss.BP_Boss_C"))
      (bind _output_get (Variables|Default|SetBoss (Utilities|Array|Get(acopy) _outactors)))
      (Transformation|SetActorRotation (Math|Rotator|FindLookatRotation _returnvalue (Transformation|GetActorLocation _output_get))))))

(event EventBeginPlay
  (CallFunction|EventSetBossandLook))

(event EventTick
  (params (DeltaSeconds :type Float%20%28single-precision%29))
  (if (Variables|Default|GetCanMove)
    (Transformation|SetActorLocation (+ (* (* 1e+03 (Transformation|GetActorForwardVector)) DeltaSeconds) (Transformation|GetActorLocation)) false false)))

(fn ConstructionScript)