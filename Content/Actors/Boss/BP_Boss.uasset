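; Boss enemy that faces the player and fires projectiles at them on a looping timeline cooldown until it dies.
; Phase enum, player and center are written to the AI Blackboard; damage, death and enemy-elimination events switch the phase and update AnimBP state.
; Non-lethal hits also broadcast a state change carrying the difficulty-based boss enemy count from the GameInstance.
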(event Custom|Event_Attack
  (Timeline|Timeline PlayFromStart
    (:Update
      (if (Default|IsDead (Variables|Default|GetBPC_HealthSystem))
        (Timeline|Timeline Stop)))
    (:Finished
      (bind _returnvalue (Game|SpawnActorfromClass "/Game/Actors/Boss/BP_BossProjectile.BP_BossProjectile_C" (Math|Conversions|ToTransform(Vector) (Transformation|GetActorLocation)) "Undefined" "MultiplyWithRoot" 0 0))
      (Default|EventSetBossandLook _returnvalue (Transformation|GetActorLocation (Variables|Default|GetPlayer)))
      (Timeline|Timeline PlayFromStart))))

(event Custom|Event_OnEnemiesEliminated
  (bind _output_get (Variables|Default|SetCurrentPhase "NewEnumerator2"))
  (AI|Components|Blackboard|SetValueasEnum (AI|GetBlackboard (Pawn|GetController)) (Variables|Default|GetKey) _output_get)
  (bind _asab_boss (Utilities|Casting|CastToAB_Boss (Components|SkeletalMesh|GetAnimInstance (Variables|Character|GetMesh))))
  (Variables|/Game/Actors/Boss/AB_Boss.AB_Boss_C|SetMovementSpeed _asab_boss 0.0))

(event Custom|Event_TakedDamage
  (params (Damage :type Float%20%28double-precision%29))
  (if (Default|IsDead (Variables|Default|GetBPC_HealthSystem))
    (bind _output_get (Variables|Default|SetCurrentPhase "NewEnumerator7"))
    (AI|Components|Blackboard|SetValueasEnum (AI|GetBlackboard (Pawn|GetController)) (Variables|Default|GetKey) _output_get)
    (bind _asab_boss (Utilities|Casting|CastToAB_Boss (Components|SkeletalMesh|GetAnimInstance (Variables|Character|GetMesh))))
    (Variables|/Game/Actors/Boss/AB_Boss.AB_Boss_C|SetIsDead _asab_boss true)
    (else
      (bind _output_get_2 (Variables|Default|SetCurrentPhase "NewEnumerator1"))
      (AI|Components|Blackboard|SetValueasEnum (AI|GetBlackboard (Pawn|GetController)) (Variables|Default|GetKey) _output_get_2)
      (Default|CallOnChangeState (.BossEnemyCountValue (Utilities|Struct|BreakSDificultData (Variables|/Game/Blueprints/BP_GI.BP_GI_C|GetGameDifficult (stale EventBeginPlay _asbp_gi)))))
      (bind _asab_boss_2 (Utilities|Casting|CastToAB_Boss (Components|SkeletalMesh|GetAnimInstance (Variables|Character|GetMesh))))
      (Variables|/Game/Actors/Boss/AB_Boss.AB_Boss_C|SetIsHitted _asab_boss_2 true)
      (Variables|/Game/Actors/Boss/AB_Boss.AB_Boss_C|SetMovementSpeed _asab_boss_2 3e+02))))

(event EventTick
  (params (DeltaSeconds :type Float%20%28single-precision%29))
  (if (not (Default|IsDead (Variables|Default|GetBPC_HealthSystem)))
    (Transformation|SetActorRotation (Math|Rotator|FindLookatRotation (Transformation|GetActorLocation) (Transformation|GetActorLocation (Variables|Default|GetPlayer))))))

(event EventBeginPlay
  (EventDispatchers|BindEventtoOnAttack (delegate Custom|Event_Attack))
  (bind _asbp_gi (Utilities|Casting|CastToBP_GI (Game|GetGameInstance)))
  (Variables|Default|SetCurrentPhase "NewEnumerator0")
  (bind _outactors (Actor|GetAllActorsOfClass "/Game/ThirdPerson/BP_ThirdPersonCharacter.BP_ThirdPersonCharacter_C"))
  (bind _array_element (Utilities|Array|ForEachLoopwithBreak _outactors)
    (:LoopBody
      (bind _output_get (Variables|Default|SetPlayer _array_element))
      (AI|Components|Blackboard|SetValueasObject (AI|GetBlackboard (Pawn|GetController)) (Variables|Default|GetPlayerKey) _output_get)
      (EventDispatchers|BindEventtoOnTakeDamage (Variables|Default|GetBPC_HealthSystem) (delegate Custom|Event_TakedDamage))
      (EventDispatchers|BindEventtoOnEnemiesEliminated (delegate Custom|Event_OnEnemiesEliminated))
      (AI|Components|Blackboard|SetValueasObject (AI|GetBlackboard (Pawn|GetController)) (Variables|Default|GetCenterKey) (Variables|Default|GetCenter)))))

(fn ConstructionScript)