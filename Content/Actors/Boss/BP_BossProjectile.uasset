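; Boss projectile actor that flies in a straight line and damages the third-person player character on overlap.
; An aim event rotates it toward a given target, then Tick moves it along its forward vector without sweep and destroys it when its lifetime runs out.
; Hits pass damage to the character's health system without destroying the projectile; overlaps with other actor types fail the cast and are ignored.
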(event Custom|Event_SetBossAndLook
  (params (Target :type Vector%20%28by%20ref%29))
  (Transformation|SetActorRotation (Math|Rotator|FindLookatRotation (Transformation|GetActorLocation) Target)))

(event Collision|EventActorBeginOverlap
  (params (OtherActor :type Actor%20Object%20Reference))
  (bind _asbp_third_person_character (Utilities|Casting|CastToBP_ThirdPersonCharacter OtherActor))
  (Utilities|IsValid _asbp_third_person_character
    (:Is%20Valid
      (Default|CallOnTakeDamage (Variables|/Game/ThirdPerson/BP_ThirdPersonCharacter.BP_ThirdPersonCharacter_C|GetBPC_HealthSystem _asbp_third_person_character) (Variables|Default|GetDamage)))
    (:Is%20Not%20Valid
      (Development|PrintString (Utilities|String|Append (Utilities|GetDisplayName OtherActor) " Hitted Boss Projectile"))
      (Actor|DestroyActor))))

(event EventTick
  (params (DeltaSeconds :type Float%20%28single-precision%29))
  (Transformation|SetActorLocation (+ (* (* (Variables|Default|GetSpeed) (Transformation|GetActorForwardVector)) DeltaSeconds) (Transformation|GetActorLocation)) false false)
  (bind _output_get (Variables|Default|SetLifetime (- (Variables|Default|GetLifetime) DeltaSeconds)))
  (if (<= _output_get 0.0)
    (Actor|DestroyActor)))

(fn ConstructionScript)