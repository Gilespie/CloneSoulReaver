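; BP_Bullet is a trap projectile that flies forward and damages the third-person character on overlap.
; Tick moves it along its forward vector without sweep and accumulates a timer, destroying the bullet once the timer reaches Delay.
; Overlapping a BP_ThirdPersonCharacter applies damage without destroying the bullet, while overlapping any other actor destroys it.
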(event Collision|EventActorBeginOverlap
  (params (OtherActor :type Actor%20Object%20Reference))
  (bind _asbp_third_person_character (Utilities|Casting|CastToBP_ThirdPersonCharacter OtherActor)
    (:then
      (Game|Damage|ApplyDamage _asbp_third_person_character (Variables|Default|GetDamage) 0 0))
    (:CastFailed
      (Actor|DestroyActor))))

(event EventTick
  (params (DeltaSeconds :type Float%20%28single-precision%29))
  (CallFunction|Move (Variables|Default|GetSpeed) DeltaSeconds)
  (bind _time (CallFunction|SetTimer DeltaSeconds))
  (if (>= _time (Variables|Default|GetDelay))
    (Variables|Default|SetTimer 0.0)
    (Actor|DestroyActor)))

(fn ConstructionScript)

(fn Move
  (params (moveSpeed :type Float%20%28double-precision%29) (deltaTime :type Float%20%28double-precision%29))
  (Transformation|SetActorLocation (+ (* (* moveSpeed (Transformation|GetActorForwardVector)) deltaTime) (Transformation|GetActorLocation)) false false))

(fn SetTimer
  (params (DeltaSeconds :type Float%20%28double-precision%29))
  (bind _output_get (Variables|Default|SetTimer (+ DeltaSeconds (Variables|Default|GetTimer))))
  (return _output_get))